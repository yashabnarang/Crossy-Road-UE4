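; Grass terrain strip that randomly scatters tree and rock accessories along its length when play begins.
; SpawnAccessory steps along Y between the terrain start and end points at a fixed spacing, rolling for a tree, then rerolling for a rock.
; Spawned actors are tracked in AccessoriesStack; the AccessoryTypes input is unused.
; Construction defers to the parent, leaving its own endpoint calculation disconnected.
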(event EventBeginPlay
  (CallFunction|SpawnAccessory (Variables|Default|GetTerrainStartPoint) (Variables|Default|GetTerrainEndPoint) 75.0 (Utilities|Array|MakeArray "NewEnumerator0" "NewEnumerator1")))

(fn ConstructionScript
  (|CallParentFunction))

(fn SpawnAccessory
  (params (StartPoint :type Vector) (EndPoint :type Vector) (AccessoryFrequency :type Float%20%28single-precision%29) (AccessoryTypes :type Array%20of%20AccessoryType%20Enums :default "NewEnumerator0"))
  (bind _returnvalue (Math|Random|RandomInteger 10))
  (for _index (range 1 (- (Math|Float|Truncate (/ (Math|Vector|Distance(Vector) StartPoint EndPoint) AccessoryFrequency)) 1))
    (if (Math|Integer|InRange(Integer) _returnvalue 6 8)
      (bind _returnvalue_2 (Game|SpawnActorfromClass "/Game/Blueprints2/Blueprints/StripAccessories/Accessory_Tree_Base.Accessory_Tree_Base_C" (Math|Transform|MakeTransform (Math|Vector|MakeVector (.x (Transformation|GetWorldLocation (Variables|Default|GetRoot))) (+ (* _index AccessoryFrequency) (.Y (Math|Vector|BreakVector StartPoint))) 0.0) "0, 0, 0" "1,1,1") "Undefined" 0 0))
      (Utilities|Array|AddUnique (Variables|Default|GetAccessoriesStack) _returnvalue_2)
      (elif (Math|Integer|InRange(Integer) _returnvalue 9 10)
        (bind _returnvalue_3 (Game|SpawnActorfromClass "/Game/Blueprints2/Blueprints/StripAccessories/Accessory_Rock_Base.Accessory_Rock_Base_C" (Math|Transform|MakeTransform (Math|Vector|MakeVector (.x (Transformation|GetWorldLocation (Variables|Default|GetRoot))) (+ (* _index AccessoryFrequency) (.Y (Math|Vector|BreakVector StartPoint))) 0.0) "0, 0, 0" "1,1,1") "Undefined" 0 0))
        (Utilities|Array|AddUnique (Variables|Default|GetAccessoriesStack) _returnvalue_3)))))