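; Base terrain strip for a Crossy Road-style game that extends the level and awards score as the player advances.
; The first player overlap of its box has Terrain_Spawner add a random strip (grass weighted over river or road) and increments the game mode score.
; It also destroys the strip four back in the spawner's TerrainStack, along with its accessories.
; The construction script derives the strip's start and end points from mesh scale.
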(event OnComponentBeginOverlap(Box)
  (params (OverlappedComponent :type Primitive%20Component%20Object%20Reference) (OtherActor :type Actor%20Object%20Reference) (OtherComp :type Primitive%20Component%20Object%20Reference) (OtherBodyIndex :type Integer) (bFromSweep :type Boolean) (SweepResult :type Hit%20Result%20Structure%20%28by%20ref%29))
  (bind _returnvalue (Math|Random|RandomBool))
  (bind _asgm_crossy_road (Utilities|Casting|CastToGM_CrossyRoad (Game|GetGameMode)))
  (bind _returnvalue_2 (Actor|GetActorOfClass (Variables|/Script/Engine.GameModeBase|GetDefaultPawnClass _asgm_crossy_road)))
  (if (== _returnvalue_2 OtherActor)
    (Utilities|FlowControl|DoOnce false
      (:Completed
        (Utilities|FlowControl|Sequence
          (:then_0
            (bind _outactors (Actor|GetAllActorsOfClass "/Game/Blueprints2/Blueprints/Terrain_Spawner.Terrain_Spawner_C"))
            (if (Math|Random|RandomBool)
              (if _returnvalue
                (Default|SpawnTerrainStripe (Utilities|Array|Get(acopy) _outactors) "/Game/Blueprints2/Blueprints/TerrainStrips/Terrain_GrassStrip.Terrain_GrassStrip_C")
                (else
                  (Default|SpawnTerrainStripe (Utilities|Array|Get(acopy) _outactors) "/Game/Blueprints2/Blueprints/TerrainStrips/Terrain_RiverStrip.Terrain_RiverStrip_C")))
              (elif _returnvalue
                (Default|SpawnTerrainStripe (Utilities|Array|Get(acopy) _outactors) "/Game/Blueprints2/Blueprints/TerrainStrips/Terrain_GrassStrip.Terrain_GrassStrip_C")
                (else
                  (Default|SpawnTerrainStripe (Utilities|Array|Get(acopy) _outactors) "/Game/Blueprints2/Blueprints/TerrainStrips/Terrain_RoadStrip.Terrain_RoadStrip_C"))))
            (Utilities|IsValid (Utilities|Array|Get(acopy) (Variables|/Game/Blueprints2/Blueprints/Terrain_Spawner.Terrain_Spawner_C|GetTerrainStack (Utilities|Array|Get(acopy) _outactors)) (- (Utilities|Array|FindItem (Variables|/Game/Blueprints2/Blueprints/Terrain_Spawner.Terrain_Spawner_C|GetTerrainStack (Utilities|Array|Get(acopy) _outactors)) self) 4))
              (:Is%20Valid
                (for _array_element (Variables|TerrainBase_C|GetAccessoriesStack (Utilities|Array|Get(acopy) (Variables|/Game/Blueprints2/Blueprints/Terrain_Spawner.Terrain_Spawner_C|GetTerrainStack (Utilities|Array|Get(acopy) _outactors)) (- (Utilities|Array|FindItem (Variables|/Game/Blueprints2/Blueprints/Terrain_Spawner.Terrain_Spawner_C|GetTerrainStack (Utilities|Array|Get(acopy) _outactors)) self) 4)))
                  (Actor|DestroyActor _array_element))
                (Actor|DestroyActor (Utilities|Array|Get(acopy) (Variables|/Game/Blueprints2/Blueprints/Terrain_Spawner.Terrain_Spawner_C|GetTerrainStack (Utilities|Array|Get(acopy) _outactors)) (- (Utilities|Array|FindItem (Variables|/Game/Blueprints2/Blueprints/Terrain_Spawner.Terrain_Spawner_C|GetTerrainStack (Utilities|Array|Get(acopy) _outactors)) self) 4))))))
          (:then_1
            (if (not (Variables|Default|GetbGavePoint))
              (Default|IncreaseScore _asgm_crossy_road)
              (Variables|Default|SetbGavePoint true))))))))

(fn ConstructionScript
  (bind _terrainstrip (Variables|Default|GetTerrainStrip))
  (bind _relativescale3d (Variables|/Script/Engine.SceneComponent|GetRelativeScale3D _terrainstrip))
  (bind _returnvalue (* (.z _relativescale3d) 5e+01))
  (Variables|Default|SetTerrainStartPoint (Math|Vector|MakeVector 0.0 (* (.y _relativescale3d) -5e+01) _returnvalue))
  (Variables|Default|SetTerrainEndPoint (Math|Vector|MakeVector 0.0 (* (.y _relativescale3d) 5e+01) _returnvalue)))