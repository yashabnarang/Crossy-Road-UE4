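; Terrain spawner that lays a fixed run of grass and road strips when play begins.
; A loop picks each strip type by index, placing a band of road between grass sections.
; SpawnTerrainStripe spawns each strip at NextTerrainTransform, then moves that transform to the new strip's Anchor location with zero rotation, chaining strips end to end.
; Each spawned strip is recorded in TerrainStack.
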(event EventBeginPlay
  (for _index (range 0 10)
    (if (Math|Integer|InRange(Integer) _index 0 1)
      (Variables|Default|SetSpawnTerrainType "NewEnumerator0" :!label _label)
      (elif (Math|Integer|InRange(Integer) _index 2 5)
        (Variables|Default|SetSpawnTerrainType "NewEnumerator1")
        (else
          (goto _label))))
    (switch Utilities|FlowControl|Switch|SwitchonTerrainType (Variables|Default|GetSpawnTerrainType)
      (:NewEnumerator0
        (CallFunction|SpawnTerrainStripe "/Game/Blueprints2/Blueprints/TerrainStrips/Terrain_GrassStrip.Terrain_GrassStrip_C"))
      (:NewEnumerator1
        (CallFunction|SpawnTerrainStripe "/Game/Blueprints2/Blueprints/TerrainStrips/Terrain_RoadStrip.Terrain_RoadStrip_C")))))

(fn ConstructionScript)

(fn SpawnTerrainStripe
  (params (Class :type Terrain%20Base%20Class%20Reference))
  (bind _returnvalue (Game|SpawnActorfromClass Class (Variables|Default|GetNextTerrainTransform) "Undefined" 0 0))
  (Variables|Default|SetNextTerrainTransform (Math|Transform|MakeTransform (Transformation|GetWorldLocation (Variables|/Game/Blueprints2/Blueprints/TerrainStrips/TerrainBase.TerrainBase_C|GetAnchor _returnvalue)) "0, 0, 0" "1,1,1"))
  (Utilities|Array|AddUnique (Variables|Default|GetTerrainStack) _returnvalue))