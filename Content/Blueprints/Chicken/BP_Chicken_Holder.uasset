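; Player character that holds a spawned, collision-free BP_Chicken model and hops it in fixed steps along four axes with WASD.
; Pressing a key turns and squashes the model; releasing turns it to any still-held direction, or hops once none remain, unless already moving.
; Each hop calls Jump, then Tick slides the capsule by fixed, unswept per-frame offsets until the step distance runs out, independent of delta time.
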(event EventBeginPlay
  ;[1 1 1] Attach Chicken Model to Holder
  (bind _returnvalue (Game|SpawnActorfromClass "/Game/Blueprints/Chicken/BP_Chicken.BP_Chicken_C" (Math|Transform|MakeTransform "0, 0, 0" "0, 0, 0" "1,1,1") "Undefined" 0 0))
  (bind _output_get (Variables|Default|SetchickenModel _returnvalue))
  (Transformation|AttachComponentToComponent _output_get (Variables|Default|GetScene) "None" "KeepRelative" "KeepRelative" "KeepRelative" true)
  (Collision|SetActorEnableCollision _output_get false))

(event EventTick
  (params (DeltaSeconds :type Float%20%28single-precision%29))
  ;[1 1 1] Tick Movement
  (if (Variables|Default|GetisMoving)
    (Transformation|AddRelativeLocation (Variables|Collision|GetCapsuleComponent) (Utilities|Select :Index (Variables|Default|Getdirection) :Option%200 "7.000000, 0, 0" :Option%201 "0,7.000000, 0" :Option%202 "-7.000000, 0, 0" :Option%203 "0,-7.000000, 0") false false)
    (bind _output_get (Variables|Default|Setdistance (+ (stale _output_get) -7.0)))
    (Math|Float|CompareFloat _output_get 0.0
      (:==
        _)
      (:<
        _))
    (Variables|Default|SetisMoving false)))

(event Input|ActionEvents|InputActionMoveForward
  (params (Key :type Key%20Structure :default "None"))
  ;[1 1 1] keyUp and keyDown (WASD)
  (:Pressed
    (CallFunction|KeyDown))
  (:Released
    (CallFunction|KeyUp)))

(event Input|ActionEvents|InputActionMoveBack
  (params (Key :type Key%20Structure :default "None"))
  ;[1 1 1] keyUp and keyDown (WASD)
  (:Pressed
    (CallFunction|KeyDown 2))
  (:Released
    (CallFunction|KeyUp 2)))

(event Input|ActionEvents|InputActionMoveRight
  (params (Key :type Key%20Structure :default "None"))
  ;[1 1 1] keyUp and keyDown (WASD)
  (:Pressed
    (CallFunction|KeyDown 3))
  (:Released
    (CallFunction|KeyUp 3)))

(event Input|ActionEvents|InputActionMoveLeft
  (params (Key :type Key%20Structure :default "None"))
  ;[1 1 1] keyUp and keyDown (WASD)
  (:Pressed
    (CallFunction|KeyDown 1))
  (:Released
    (CallFunction|KeyUp 1)))

(fn ConstructionScript)

(fn Move
  (params (Direction :type Integer))
  (Utilities|Array|SetArrayElem (Variables|Default|GetkeyIsDown) Direction false)
  (Transformation|SetActorRelativeTransform (Variables|Default|GetchickenModel) (Math|Transform|MakeTransform "0, 0, 0" (Utilities|Select :Index Direction :Option%200 "0, 0, 0" :Option%201 "0,90.000000, 0" :Option%202 "0,180.000000, 0" :Option%203 "0,270.000000, 0") "1,1,1") false false)
  (Character|Jump)
  (Variables|Default|Setdistance 1.1e+02)
  (Variables|Default|Setdirection Direction)
  (Variables|Default|SetisMoving true))

(fn KeyUp
  (params (Direction :type Integer))
  (Utilities|Array|SetArrayElem (Variables|Default|GetkeyIsDown) Direction false)
  (LocalVariables|SetKeyStillDown false)
  ;[1 1 1] Loop to ensure chicken jumps in the correct direction
  (bind (_array_element _array_index) (Utilities|Array|ForEachLoopwithBreak (Variables|Default|GetkeyIsDown) :!label _label)
    (:LoopBody
      (if _array_element
        (LocalVariables|SetKeyStillDown true)
        (Transformation|SetActorRotation (Variables|Default|GetchickenModel) (Utilities|Select :Index _array_index :Option%200 "0, 0, 0" :Option%201 "0,90.000000, 0" :Option%202 "0,180.000000, 0" :Option%203 "0.000000,270.000000, 0"))
        (goto _label Break)))
    (:Completed
      ;[1 1 1] Move (Jump) in correct direction
      (if (not (LocalVariables|GetKeyStillDown))
        (if (Variables|Default|GetisMoving)
          ;[1 1 1] Ensure Chicken is not squished and in correct direction
          (Transformation|SetActorRelativeTransform (Variables|Default|GetchickenModel) (Math|Transform|MakeTransform "0, 0, 0" (Utilities|Select :Index Direction :Option%200 "0, 0, 0" :Option%201 "0,90.000000, 0" :Option%202 "0,180.000000, 0" :Option%203 "0.000000,270.000000, 0") "1,1,1") false false)
          (else
            (CallFunction|Move Direction)))))))

(fn KeyDown
  (params (Direction :type Integer))
  (Transformation|SetActorRelativeTransform (Variables|Default|GetchickenModel) (Math|Transform|MakeTransform "0, 0, 0" (Utilities|Select :Index Direction :Option%200 "0, 0, 0" :Option%201 "0,90.000000, 0" :Option%202 "0,180.000000, 0" :Option%203 "0,270.000000, 0") "1,0.800000,1.000000") false false) ; Squishs The Chicken
  (Utilities|Array|SetArrayElem (Variables|Default|GetkeyIsDown) Direction true))