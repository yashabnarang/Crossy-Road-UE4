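; Train accessory for a Crossy Road-style game that acts as a lethal moving hazard for the chicken player.
; On BeginPlay, nested coin flips either play one of two train sounds, set projectile movement speed and destroy it after five seconds, or skip all three.
; Overlapping the chicken with the collision component plays a death sound, flattens the chicken, then pauses and shows the end screen with the GameMode score.
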(event OnComponentBeginOverlap(VehicleCollision)
  (params (OverlappedComponent :type Primitive%20Component%20Object%20Reference) (OtherActor :type Actor%20Object%20Reference) (OtherComp :type Primitive%20Component%20Object%20Reference) (OtherBodyIndex :type Integer) (bFromSweep :type Boolean) (SweepResult :type Hit%20Result%20Structure%20%28by%20ref%29))
  (bind _asbp_chicken_holder (Utilities|Casting|CastToBP_Chicken_Holder OtherActor))
  (Audio|PlaySoundatLocation "/Game/Models/Sounds/sounds/chicken_die1_Cue.chicken_die1_Cue" "0, 0, 0" "0, 0, 0" 1.0 1.0 0.0 0 0 0)
  (Transformation|SetWorldScale3D (Variables|/Game/Blueprints/Chicken/BP_Chicken_Holder.BP_Chicken_Holder_C|GetChicken _asbp_chicken_holder) "1.000000,1.000000,0.100000")
  (Utilities|FlowControl|Delay 0.3)
  (Game|SetGamePaused true)
  (bind _returnvalue (UserInterface|CreateWidget "/Game/Widgets/WB_Endscreen.WB_Endscreen_C" 0 (Variables|/Game/Blueprints/GM_CrossyRoad.GM_CrossyRoad_C|GetScore (.AsGM%20Crossy%20Road (Utilities|Casting|CastToGM_CrossyRoad (Game|GetGameMode))))))
  (UserInterface|Viewport|AddtoViewport _returnvalue 0))

(event EventBeginPlay
  (bind _returnvalue (Math|Random|RandomBool))
  (bind _projectilemovement (Variables|Default|GetProjectileMovement))
  (|CallParentFunction)
  (if (Math|Random|RandomBool)
    (if _returnvalue
      (Audio|PlaySoundatLocation "/Game/Models/Sounds/sounds/train_move1_Cue.train_move1_Cue" "0, 0, 0" "0, 0, 0" 1.0 1.0 0.0 0 0 0)
      (Variables|/Script/Engine.ProjectileMovementComponent|SetInitialSpeed _projectilemovement (Variables|Default|GetSpeed) :!label _label)
      (Variables|/Script/Engine.ProjectileMovementComponent|SetMaxSpeed _projectilemovement (Variables|Default|GetSpeed))
      (Utilities|FlowControl|Delay 5.0)
      (Actor|DestroyActor))
    (elif _returnvalue
      (Audio|PlaySoundatLocation "/Game/Models/Sounds/sounds/train_move2_Cue.train_move2_Cue" "0, 0, 0" "0, 0, 0" 1.0 1.0 0.0 0 0 0)
      (goto _label))))

(event Collision|EventActorBeginOverlap
  (params (OtherActor :type Actor%20Object%20Reference))
  (|CallParentFunction OtherActor) ; This node is disabled and will not be called.\nDrag off pins to build functionality.
)

(event EventTick
  (params (DeltaSeconds :type Float%20%28single-precision%29))
  (|CallParentFunction DeltaSeconds) ; This node is disabled and will not be called.\nDrag off pins to build functionality.
)

(fn ConstructionScript
  (|CallParentFunction))