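; Railroad terrain strip that periodically sends trains across its width from one side, chosen at random on BeginPlay.
; A non-looping timer re-arms itself with a new random delay after each spawn attempt.
; Each attempt must pass two random checks, then spawns an Accessory_Train at the strip's start or end point, facing across it, and records it in AccessoriesStack.
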(event Custom|SpawnTrain
  (CallFunction|SpawnAccessory (Variables|Default|GetSpawnTrainFromLeft))
  (bind _returnvalue (Utilities|Time|SetTimerbyEvent (delegate Custom|SpawnTrain) (Math|Random|RandomFloatinRange 1.5 3.0)))
  (Variables|Default|SetTrain%20Spawn%20Timer _returnvalue))

(event EventBeginPlay
  (Variables|Default|SetSpawnTrainFromLeft (Math|Random|RandomBool))
  (bind _returnvalue (Utilities|Time|SetTimerbyEvent (delegate Custom|SpawnTrain) (Math|Random|RandomFloatinRange 1.5 3.0)))
  (Variables|Default|SetTrain%20Spawn%20Timer _returnvalue))

(fn ConstructionScript
  (|CallParentFunction))

(fn SpawnAccessory
  (params (SpawnFromLeft :type Boolean))
  (bind _root (Variables|Default|GetRoot))
  (bind _returnvalue (Transformation|GetWorldLocation _root))
  (if (Math|Random|RandomBool)
    (if SpawnFromLeft
      (LocalVariables|SetSpawn%20Location (Math|Vector|MakeVector (.x _returnvalue) (.y (Variables|Default|GetTerrainEndPoint)) 0.0))
      (LocalVariables|SetSpawnRotation "0,-90.000000, 0")
      (else
        (LocalVariables|SetSpawn%20Location (Math|Vector|MakeVector (.x _returnvalue) (.y (Variables|Default|GetTerrainStartPoint)) 0.0))
        (LocalVariables|SetSpawnRotation "0,90.000000, 0")))
    (if (Math|Integer|InRange(Integer) (Math|Random|RandomInteger 10) 0 7)
      (bind _returnvalue_2 (Game|SpawnActorfromClass "/Game/Blueprints2/Blueprints/StripAccessories/Accessory_Train.Accessory_Train_C" (Math|Transform|MakeTransform (LocalVariables|GetSpawn%20Location) (LocalVariables|GetSpawnRotation) "1,1,1") "Undefined" 0 0))
      (Utilities|Array|AddUnique (Variables|Default|GetAccessoriesStack) _returnvalue_2))))