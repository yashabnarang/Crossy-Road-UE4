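; Road terrain strip that spawns car and truck traffic crossing it in one direction, chosen at random on BeginPlay.
; A one-shot timer re-arms itself with a random delay after each spawn attempt, and each attempt has an even chance of producing a vehicle.
; Vehicles, weighted toward cars over trucks, appear at a strip endpoint with matching yaw and are recorded in AccessoriesStack.
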(event Custom|SpawnVehicle
  (CallFunction|SpawnAccessory (Variables|Default|GetSpawnVehicleFromLeft))
  (bind _returnvalue (Utilities|Time|SetTimerbyEvent (delegate Custom|SpawnVehicle) (Math|Random|RandomFloatinRange 1.5 3.0)))
  (Variables|Default|SetVehicle%20Spawn%20Timer _returnvalue))

(event EventBeginPlay
  (Variables|Default|SetSpawnVehicleFromLeft (Math|Random|RandomBool))
  (bind _returnvalue (Utilities|Time|SetTimerbyEvent (delegate Custom|SpawnVehicle) (Math|Random|RandomFloatinRange 1.5 3.0)))
  (Variables|Default|SetVehicle%20Spawn%20Timer _returnvalue))

(fn ConstructionScript
  (|CallParentFunction))

(fn SpawnAccessory
  (params (SpawnFromLeft :type Boolean))
  (bind _root (Variables|Default|GetRoot))
  (bind _returnvalue (Transformation|GetWorldLocation _root))
  (if (Math|Random|RandomBool)
    (if SpawnFromLeft
      (LocalVariables|SetSpawn%20Location (Math|Vector|MakeVector (.x _returnvalue) (.y (Variables|Default|GetTerrainEndPoint)) 0.0))
      (LocalVariables|SetSpawnRotation "0,-90.000000, 0")
      (else
        (LocalVariables|SetSpawn%20Location (Math|Vector|MakeVector (.x _returnvalue) (.y (Variables|Default|GetTerrainStartPoint)) 0.0))
        (LocalVariables|SetSpawnRotation "0,90.000000, 0")))
    (if (Math|Integer|InRange(Integer) (Math|Random|RandomInteger 10) 0 7)
      (bind _returnvalue_2 (Game|SpawnActorfromClass "/Game/Blueprints2/Blueprints/StripAccessories/Accessory_Vehicle_Car.Accessory_Vehicle_Car_C" (Math|Transform|MakeTransform (LocalVariables|GetSpawn%20Location) (LocalVariables|GetSpawnRotation) "1,1,1") "Undefined" 0 0))
      (Utilities|Array|AddUnique (Variables|Default|GetAccessoriesStack) _returnvalue_2)
      (else
        (bind _returnvalue_3 (Game|SpawnActorfromClass "/Game/Blueprints2/Blueprints/StripAccessories/Accessory_Vehicle_Truck.Accessory_Vehicle_Truck_C" (Math|Transform|MakeTransform (LocalVariables|GetSpawn%20Location) (LocalVariables|GetSpawnRotation) "1,1,1") "Undefined" 0 0))
        (Utilities|Array|AddUnique (Variables|Default|GetAccessoriesStack) _returnvalue_3)))))