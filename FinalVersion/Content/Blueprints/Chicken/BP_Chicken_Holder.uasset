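; Player-controlled chicken that hops in fixed steps along the world X and Y axes, Crossy Road style.
; Axis input past a deadzone starts a half-second cooldown, yaws the chicken and plays a random cluck.
; A timeline lerps the capsule to the target, with a separate track for the hop arc.
; Separate KeyDown, KeyUp and Move functions implement squash-and-release jumping, but the event graph never calls them.
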(event Custom|SetMovementCooldown
  ;[0 1 0.1289] COOLDOWN FOR INPUTS
  (Utilities|FlowControl|DoOnce false :!label _label
    (:Completed
      (Variables|Default|SetCanMove false)
      (Utilities|FlowControl|Delay 0.5)
      (Variables|Default|SetCanMove true)
      (goto _label Reset))))

(event Custom|MoveToTargetLocation
  (params (Upwards :type Float%20%28single-precision%29) (Rightwards :type Float%20%28single-precision%29) (MoveFactor :type Float%20%28single-precision%29))
  (bind _capsulecomponent (Variables|Collision|GetCapsuleComponent))
  (bind _returnvalue (Transformation|GetWorldLocation _capsulecomponent))
  ;[0 1 0.2357] BASIC MOVE JUMP
  (Variables|Default|SetInitialLocation _returnvalue)
  (Variables|Default|SetFinalLocation (+ _returnvalue (Math|Vector|MakeVector (* Upwards MoveFactor) (* Rightwards MoveFactor) 0.0)))
  (bind (_direction _movement _jump) (Timeline|Timeline_0 PlayFromStart)
    (:Update
      (Transformation|SetWorldLocation (Variables|Collision|GetCapsuleComponent) (Math|Vector|Lerp(Vector) (Math|Vector|MakeVector (.x (Variables|Default|GetInitialLocation)) (.y (Variables|Default|GetInitialLocation)) (Math|Float|Lerp (.z (Variables|Default|GetInitialLocation)) (+ (.z (Variables|Default|GetInitialLocation)) 5e+01) _jump)) (Math|Vector|MakeVector (.x (Variables|Default|GetFinalLocation)) (.y (Variables|Default|GetFinalLocation)) (Math|Float|Lerp (.z (Variables|Default|GetInitialLocation)) (+ (.z (Variables|Default|GetInitialLocation)) 5e+01) _jump)) _movement) false false))))

(event Input|AxisEvents|InputAxisMoveUp
  (params (AxisValue :type Float%20%28single-precision%29))
  ;[0.1075 1 0.08636] DETECT AND SEND INPUT AXIS
  (if (and (> (Math|Float|Absolute(Float) AxisValue) 0.3) (Variables|Default|GetCanMove))
    (CallFunction|SetMovementCooldown)
    (CallFunction|MovetoTargetLocation AxisValue 0.0 1e+02)
    (if (Math|Float|InRange(Float) AxisValue 1.0 1.0)
      (Variables|Default|SetzRotation 0)
      (else
        (Variables|Default|SetzRotation 180)))
    (Transformation|SetRelativeRotation (Variables|Default|GetChicken) (Math|Rotator|MakeRotator 0.0 0.0 (Math|Conversions|ToFloat(Integer) (Variables|Default|GetzRotation))) false false)
    ;[0.351 0.1703 1] Chicken Sounds
    (Audio|PlaySoundatLocation (Utilities|Select :Index (Math|Random|RandomIntegerinRange 0 2) :Option%200 "/Game/Models/Sounds/sounds/chicken_cluck1_Cue.chicken_cluck1_Cue" :Option%201 "/Game/Models/Sounds/sounds/chicken_cluck2_Cue.chicken_cluck2_Cue" :Option%202 "/Game/Models/Sounds/sounds/chicken_cluck3.chicken_cluck3" :Option%203 0) "0, 0, 0" "0, 0, 0" 1.0 1.0 0.0 0 0 0)))

(event Input|AxisEvents|InputAxisMoveRight
  (params (AxisValue :type Float%20%28single-precision%29))
  ;[0.1075 1 0.08636] DETECT AND SEND INPUT AXIS
  (if (and (> (Math|Float|Absolute(Float) AxisValue) 0.3) (Variables|Default|GetCanMove))
    (CallFunction|SetMovementCooldown)
    (CallFunction|MovetoTargetLocation 0.0 AxisValue 1e+02)
    (if (Math|Float|InRange(Float) AxisValue 1.0 1.0)
      (Variables|Default|SetzRotation 90)
      (else
        (Variables|Default|SetzRotation 270)))
    (Transformation|SetRelativeRotation (Variables|Default|GetChicken) (Math|Rotator|MakeRotator 0.0 0.0 (Math|Conversions|ToFloat(Integer) (Variables|Default|GetzRotation))) false false)
    ;[0.351 0.1703 1] Chicken Sounds
    (Audio|PlaySoundatLocation (Utilities|Select :Index (Math|Random|RandomIntegerinRange 0 2) :Option%200 "/Game/Models/Sounds/sounds/chicken_cluck1_Cue.chicken_cluck1_Cue" :Option%201 "/Game/Models/Sounds/sounds/chicken_cluck2_Cue.chicken_cluck2_Cue" :Option%202 "/Game/Models/Sounds/sounds/chicken_cluck3.chicken_cluck3" :Option%203 0) "0, 0, 0" "0, 0, 0" 1.0 1.0 0.0 0 0 0)))

(fn ConstructionScript)

(fn Move
  (params (Direction :type Integer))
  (Utilities|Array|SetArrayElem (Variables|Default|GetkeyIsDown) Direction false)
  (Transformation|SetActorRelativeTransform (Variables|Default|GetchickenModel) (Math|Transform|MakeTransform "0, 0, 0" (Utilities|Select :Index Direction :Option%200 "0, 0, 0" :Option%201 "0,90.000000, 0" :Option%202 "0,180.000000, 0" :Option%203 "0,270.000000, 0") "1,1,1") false false)
  (Character|Jump)
  (Variables|Default|Setdistance 98.050003)
  (Variables|Default|Setdirection Direction)
  (Variables|Default|SetisMoving true))

(fn KeyUp
  (params (Direction :type Integer))
  (Utilities|Array|SetArrayElem (Variables|Default|GetkeyIsDown) Direction false)
  (LocalVariables|SetKeyStillDown false)
  ;[1 1 1] Loop to ensure chicken jumps in the correct direction
  (bind (_array_element _array_index) (Utilities|Array|ForEachLoopwithBreak (Variables|Default|GetkeyIsDown) :!label _label)
    (:LoopBody
      (if _array_element
        (LocalVariables|SetKeyStillDown true)
        (Transformation|SetActorRotation (Variables|Default|GetchickenModel) (Utilities|Select :Index _array_index :Option%200 "0, 0, 0" :Option%201 "0,90.000000, 0" :Option%202 "0,180.000000, 0" :Option%203 "0.000000,270.000000, 0"))
        (goto _label Break)))
    (:Completed
      ;[1 1 1] Move (Jump) in correct direction
      (if (not (LocalVariables|GetKeyStillDown))
        (if (Variables|Default|GetisMoving)
          ;[1 1 1] Ensure Chicken is not squished and in correct direction
          (Transformation|SetActorRelativeTransform (Variables|Default|GetchickenModel) (Math|Transform|MakeTransform "0, 0, 0" (Utilities|Select :Index Direction :Option%200 "0, 0, 0" :Option%201 "0,90.000000, 0" :Option%202 "0,180.000000, 0" :Option%203 "0.000000,270.000000, 0") "1,1,1") false false)
          (else
            (CallFunction|Move Direction)))))))

(fn KeyDown
  (params (Direction :type Integer))
  (Transformation|SetActorRelativeTransform (Variables|Default|GetchickenModel) (Math|Transform|MakeTransform "0, 0, 0" (Utilities|Select :Index Direction :Option%200 "0, 0, 0" :Option%201 "0,90.000000, 0" :Option%202 "0,180.000000, 0" :Option%203 "0,270.000000, 0") "1,0.800000,1.000000") false false) ; Squishs The Chicken
  (Utilities|Array|SetArrayElem (Variables|Default|GetkeyIsDown) Direction true))